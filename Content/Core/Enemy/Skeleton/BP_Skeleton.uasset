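; Skeleton enemy that reacts to contact through a sphere and takes spell damage through its capsule.
; Sphere overlaps with non-skeletons briefly disable the sphere's collision as a cooldown, apply a health change via StatsComponent lookup, and destroy the other actor if that health is depleted.
; Capsule overlaps with BP_SpellTestMaster apply the spell's damage to its StatsComponent; at zero health it plays a death animation, then destroys itself after a delay.
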(event OnComponentBeginOverlap(Sphere)
  (params (OverlappedComponent :type Primitive%20Component%20Object%20Reference) (OtherActor :type Actor%20Object%20Reference) (OtherComp :type Primitive%20Component%20Object%20Reference) (OtherBodyIndex :type Integer) (bFromSweep :type Boolean) (SweepResult :type Hit%20Result%20Structure%20%28by%20ref%29))
  (bind _returnvalue (Actor|GetComponentbyClass "/Script/HandGameplay.StatsComponent"))
  (if (!= (Utilities|GetClass OtherActor) "BP_Skeleton_C")
    (CallFunction|Cooldown)
    (Class|StatsComponent|HealthChange _returnvalue 1e+01 true)
    (if (<= (Class|StatsComponent|GetCurrentHealth _returnvalue) 0.0)
      (Actor|DestroyActor OtherActor))))

(event OnComponentBeginOverlap(CapsuleComponent)
  (params (OverlappedComponent :type Primitive%20Component%20Object%20Reference) (OtherActor :type Actor%20Object%20Reference) (OtherComp :type Primitive%20Component%20Object%20Reference) (OtherBodyIndex :type Integer) (bFromSweep :type Boolean) (SweepResult :type Hit%20Result%20Structure%20%28by%20ref%29))
  (bind _asbp_spell_test_master (Utilities|Casting|CastToBP_SpellTestMaster OtherActor))
  (Class|StatsComponent|HealthChange (Variables|Default|GetStatsComponent) (Variables|/Game/Core/Spells/BP_SpellTestMaster.BP_SpellTestMaster_C|GetDamage _asbp_spell_test_master) true)
  (if (<= (Class|StatsComponent|GetCurrentHealth (Variables|Default|GetStatsComponent)) 0.0)
    (Components|Animation|PlayAnimation (Variables|Character|GetMesh) "/Game/UndeadPack/SkeletonEnemy/Animations/Anim_Death.Anim_Death" false)
    (Utilities|FlowControl|Delay 5.0)
    (Actor|DestroyActor)))

(event Custom|Cooldown
  (Collision|SetCollisionEnabled (Variables|Default|GetSphere) "NoCollision")
  (Utilities|FlowControl|Delay 0.5)
  (Collision|SetCollisionEnabled (Variables|Default|GetSphere) "QueryAndPhysics"))

(event EventBeginPlay
  (Development|PrintString "zyje" true true "(R=0.000000,G=0.660000,B=1.000000,A=1.000000)" 1e+01))

(event Collision|EventActorBeginOverlap
  (params (OtherActor :type Actor%20Object%20Reference)))

(event EventTick
  (params (DeltaSeconds :type Float%20%28single-precision%29)))

(fn ConstructionScript)