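; BP_Training is a training target that takes spell hits and shows death by turning red.
; Overlaps from BP_SpellTestMaster actors pass their damage to StatsComponent and print current health.
; The death event swaps the mesh material, then unbinds itself, so it responds only once.
; Full heal resets a DoOnce that the hit path enters, so the default material returns on a hit rather than on the heal itself.
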(event OnComponentBeginOverlap(CapsuleComponent)
  (params (OverlappedComponent :type Primitive%20Component%20Object%20Reference) (OtherActor :type Actor%20Object%20Reference) (OtherComp :type Primitive%20Component%20Object%20Reference) (OtherBodyIndex :type Integer) (bFromSweep :type Boolean) (SweepResult :type Hit%20Result%20Structure%20%28by%20ref%29))
  (bind _asbp_spell_test_master (Utilities|Casting|CastToBP_SpellTestMaster OtherActor))
  (Class|StatsComponent|HealthChange (Variables|Default|GetStatsComponent) (Variables|/Game/Core/Spells/BP_SpellTestMaster.BP_SpellTestMaster_C|GetDamage _asbp_spell_test_master) true)
  (Development|PrintString (Utilities|String|ToString(Float) (Class|StatsComponent|GetCurrentHealth (Variables|Default|GetStatsComponent))) true true "(R=0.000000,G=0.660000,B=1.000000,A=1.000000)" 1e+01)
  (Utilities|FlowControl|DoOnce false
    (:Completed
      (Rendering|Material|SetMaterial (Variables|Character|GetMesh) 0 "/Engine/Tutorial/SubEditors/TutorialAssets/Character/TutorialTPP_Mat.TutorialTPP_Mat"))))

(event Custom|CustomEvent
  (Development|PrintString "Died")
  (Rendering|Material|SetMaterial (Variables|Character|GetMesh) 0 "/AnimationSharing/AnimSharingRed.AnimSharingRed")
  (EventDispatchers|UnbindEventfromOnDeath (Variables|Default|GetStatsComponent) (delegate Custom|CustomEvent)))

(event Custom|Reset%20Material
  (Utilities|FlowControl|DoOnce false) ; enters at Reset
)

(event EventBeginPlay
  (bind _statscomponent (Variables|Default|GetStatsComponent))
  (EventDispatchers|BindEventtoOnDeath _statscomponent (delegate Custom|CustomEvent))
  (EventDispatchers|BindEventtoOnFullyHealed _statscomponent (delegate Custom|Reset%20Material)))

(fn ConstructionScript)